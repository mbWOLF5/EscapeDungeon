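; BP_Cell_Door is an interactive metal cell door that the player swings open and shut when in range.
; A box trigger sets PlayerRange and the first-person character's interaction flag, refreshing its crosshair on enter and exit.
; The Interaction event toggles the state, plays a sound and runs or reverses a yaw timeline.
; The mesh switches to overlap-only collision while moving, then back to blocking when the timeline finishes.
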(event `/Game/FirstPerson/Blueprints/BPI/BPI_Interaction.Interaction`
  (bind _returnvalue (`self.K2_GetActorLocation`))
  (if (`self.PlayerRange`)
    (if (`self.DoorOpen?`)
      (set `self.DoorOpen?` false)
      (`GameplayStatics.PlaySoundAtLocation` "/Game/Blueprints/Sounds/SoundCue/SC_Door_Metal_Close.SC_Door_Metal_Close" _returnvalue (struct) 1.0 1.0 0.0 null null null null)
      (`PrimitiveComponent.SetCollisionProfileName` (`self.SM_Cell_Door`) "OverlapAllDynamic" true)
      (bind (_direction _openvalue) (`Timeline|Timeline_Open` :!via `Reverse` :!label _label)
        (:`Update`
          (`SceneComponent.K2_SetRelativeRotation` (`self.SM_Cell_Door`) (`KismetMathLibrary.MakeRotator` 0.0 0.0 _openvalue) false false))
        (:`Finished`
          (`PrimitiveComponent.SetCollisionProfileName` (`self.SM_Cell_Door`) "BlockAllDynamic" true)))
      (else
        (set `self.DoorOpen?` true)
        (`GameplayStatics.PlaySoundAtLocation` "/Game/Blueprints/Sounds/SoundCue/SC_Door_Metal_Open.SC_Door_Metal_Open" _returnvalue (struct) 1.0 1.0 0.0 null null null null)
        (`PrimitiveComponent.SetCollisionProfileName` (`self.SM_Cell_Door`) "OverlapAllDynamic" true)
        (goto _label)))))

(event `self.BoxColiider.OnComponentBeginOverlap`
  (params (OverlappedComponent :type "PrimitiveComponent Object Reference") (OtherActor :type "Actor Object Reference") (OtherComp :type "PrimitiveComponent Object Reference") (OtherBodyIndex :type Integer) (bFromSweep :type Boolean) (SweepResult :type "HitResult Structure (by ref)"))
  (bind _returnvalue (`GameplayStatics.GetPlayerCharacter` 0))
  (if (== OtherActor _returnvalue)
    (bind _asbp_first_person_character (cast `/Game/FirstPerson/Blueprints/BP_FirstPersonCharacter` _returnvalue))
    (set `/Game/FirstPerson/Blueprints/BP_FirstPersonCharacter.Interraction?` true _asbp_first_person_character)
    (set `self.PlayerRange` true)
    (`/Game/FirstPerson/Blueprints/BP_FirstPersonCharacter.crosshair` _asbp_first_person_character)))

(event `self.BoxColiider.OnComponentEndOverlap`
  (params (OverlappedComponent :type "PrimitiveComponent Object Reference") (OtherActor :type "Actor Object Reference") (OtherComp :type "PrimitiveComponent Object Reference") (OtherBodyIndex :type Integer))
  (bind _returnvalue (`GameplayStatics.GetPlayerCharacter` 0))
  (if (== OtherActor _returnvalue)
    (bind _asbp_first_person_character (cast `/Game/FirstPerson/Blueprints/BP_FirstPersonCharacter` _returnvalue))
    (set `/Game/FirstPerson/Blueprints/BP_FirstPersonCharacter.Interraction?` false _asbp_first_person_character)
    (set `self.PlayerRange` false)
    (`/Game/FirstPerson/Blueprints/BP_FirstPersonCharacter.crosshair` _asbp_first_person_character)))

(fn `UserConstructionScript`)