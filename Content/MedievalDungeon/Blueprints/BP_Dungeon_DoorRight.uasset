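; BP_Dungeon_DoorRight is an interactive dungeon door that swings open and closed.
; A box collider flags when the first-person character is in range, which lets the Interaction event toggle the door.
; A single timeline plays or reverses to drive the mesh's negated relative yaw.
; The mesh switches to overlap collision while moving and back to blocking when the timeline finishes.
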(event `/Game/FirstPerson/Blueprints/BPI/BPI_Interaction.Interaction`
  (bind _sm_doorway_large_door_left (`self.SM_DoorWay_Large_Door_Left`))
  (if (`self.PlayerRange`)
    (if (`self.DoorOpen?`)
      (set `self.DoorOpen?` false)
      (`PrimitiveComponent.SetCollisionProfileName` _sm_doorway_large_door_left "OverlapAllDynamic" true)
      (bind (_direction _openvalue) (`Timeline|Timeline` :!via `Reverse` :!label _label)
        (:`Update`
          (`SceneComponent.K2_SetRelativeRotation` (`self.SM_DoorWay_Large_Door_Left`) (`KismetMathLibrary.MakeRotator` 0.0 0.0 (* _openvalue -1.0)) false false))
        (:`Finished`
          (`PrimitiveComponent.SetCollisionProfileName` (`self.SM_DoorWay_Large_Door_Left`) "BlockAllDynamic" true)))
      (else
        (set `self.DoorOpen?` true)
        (`PrimitiveComponent.SetCollisionProfileName` _sm_doorway_large_door_left "OverlapAllDynamic" true)
        (goto _label)))))

(event `self.BoxCollider.OnComponentBeginOverlap`
  (params (OverlappedComponent :type "PrimitiveComponent Object Reference") (OtherActor :type "Actor Object Reference") (OtherComp :type "PrimitiveComponent Object Reference") (OtherBodyIndex :type Integer) (bFromSweep :type Boolean) (SweepResult :type "HitResult Structure (by ref)"))
  (cast `/Game/FirstPerson/Blueprints/BP_FirstPersonCharacter` OtherActor)
  (if true
    (set `self.PlayerRange` true)))

(event `self.BoxCollider.OnComponentEndOverlap`
  (params (OverlappedComponent :type "PrimitiveComponent Object Reference") (OtherActor :type "Actor Object Reference") (OtherComp :type "PrimitiveComponent Object Reference") (OtherBodyIndex :type Integer))
  (cast `/Game/FirstPerson/Blueprints/BP_FirstPersonCharacter` OtherActor)
  (if true
    (set `self.PlayerRange` false)))

(fn `UserConstructionScript`)