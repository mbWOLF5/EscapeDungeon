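; Locked double-door Blueprint for the dungeon's final door, which the player can open and close once Open_Door flags the key as taken.
; Interaction works only while the first-person character is inside BoxCollider, adding a key sound to the first opening.
; A Timeline plays or reverses to swing both leaves in mirrored yaw.
; The right leaf switches to overlap collision during movement, and both leaves return to blocking when it finishes.
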(event `Open_Door`
  (set `self.KeyTaken?` true))

(event `/Game/FirstPerson/Blueprints/BPI/BPI_Interaction.Interaction`
  (bind _returnvalue (`self.K2_GetActorLocation`))
  (bind _sm_doorway_large_door_right (`self.SM_DoorWay_Large_Door_Right`))
  (if (`self.KeyTaken?`)
    (if (`self.PlayerRange`)
      (if (`self.DoorOpen?`)
        (set `self.DoorOpen?` false)
        (`GameplayStatics.PlaySoundAtLocation` "/Game/Blueprints/Sounds/SoundCue/SC_Door_Wood_Close.SC_Door_Wood_Close" _returnvalue (struct) 1.0 1.0 0.0 null null null null)
        (`PrimitiveComponent.SetCollisionProfileName` _sm_doorway_large_door_right "OverlapAllDynamic" true)
        (`PrimitiveComponent.SetCollisionProfileName` (`self.SM_DoorWay_Large_Door_Right`) "OverlapAllDynamic" true)
        (bind (_direction _openvalue) (`Timeline|Timeline` :!via `Reverse` :!label _label)
          (:`Update`
            (`SceneComponent.K2_SetRelativeRotation` (`self.SM_DoorWay_Large_Door_Right`) (`KismetMathLibrary.MakeRotator` 0.0 0.0 _openvalue) false false)
            (`SceneComponent.K2_SetRelativeRotation` (`self.SM_DoorWay_Large_Door_Left`) (`KismetMathLibrary.MakeRotator` 0.0 0.0 (* _openvalue -1.0)) false false))
          (:`Finished`
            (`PrimitiveComponent.SetCollisionProfileName` (`self.SM_DoorWay_Large_Door_Right`) "BlockAllDynamic" true)
            (`PrimitiveComponent.SetCollisionProfileName` (`self.SM_DoorWay_Large_Door_Left`) "BlockAllDynamic" true)))
        (else
          (set `self.DoorOpen?` true)
          (if (`self.Key?`)
            (`GameplayStatics.PlaySoundAtLocation` "/Game/Blueprints/Sounds/Sounds/Key/KeyChain_BW8848.KeyChain_BW8848" _returnvalue (struct) 1.0 1.0 0.0 null null null null)
            (`GameplayStatics.PlaySoundAtLocation` "/Game/Blueprints/Sounds/SoundCue/SC_Door_Wood_Open.SC_Door_Wood_Open" _returnvalue (struct) 1.0 1.0 0.0 null null null null)
            (set `self.Key?` false)
            (else
              (`GameplayStatics.PlaySoundAtLocation` "/Game/Blueprints/Sounds/SoundCue/SC_Door_Wood_Open.SC_Door_Wood_Open" _returnvalue (struct) 1.0 1.0 0.0 null null null null)))
          (`PrimitiveComponent.SetCollisionProfileName` _sm_doorway_large_door_right "OverlapAllDynamic" true)
          (`PrimitiveComponent.SetCollisionProfileName` (`self.SM_DoorWay_Large_Door_Right`) "OverlapAllDynamic" true)
          (goto _label))))))

(event `self.BoxCollider.OnComponentBeginOverlap`
  (params (OverlappedComponent :type "PrimitiveComponent Object Reference") (OtherActor :type "Actor Object Reference") (OtherComp :type "PrimitiveComponent Object Reference") (OtherBodyIndex :type Integer) (bFromSweep :type Boolean) (SweepResult :type "HitResult Structure (by ref)"))
  (cast `/Game/FirstPerson/Blueprints/BP_FirstPersonCharacter` OtherActor)
  (if true
    (set `self.PlayerRange` true)))

(event `self.BoxCollider.OnComponentEndOverlap`
  (params (OverlappedComponent :type "PrimitiveComponent Object Reference") (OtherActor :type "Actor Object Reference") (OtherComp :type "PrimitiveComponent Object Reference") (OtherBodyIndex :type Integer))
  (cast `/Game/FirstPerson/Blueprints/BP_FirstPersonCharacter` OtherActor)
  (if true
    (set `self.PlayerRange` false)))

(fn `UserConstructionScript`)